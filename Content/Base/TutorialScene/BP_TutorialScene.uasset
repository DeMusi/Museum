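; Tutorial scene Blueprint for VR that walks an entering motion controller pawn through logos, a test and a hotspot before unlocking teleporting.
; On player entry it caches the pawn's face-image widget, binds dispatchers, shows two timed logos, then starts and opens the test.
; Finishing the test closes it and reveals the hotspot after a short delay.
; Activating the hotspot hides it, enables controller teleport and shows a gamepad image, which hides when the player leaves.
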(event Custom|TutorialTestCompleted
  (Default|EventClose (Variables|Default|GetBP_Test))
  (Utilities|FlowControl|Delay 1.0)
  (Default|EventShow (Variables|Default|GetBP_Hotspot)))

(event Custom|TutorialHotspotActivated
  (bind _pawnwbpfaceimg (Variables|Default|GetPawnWBPFaceImg))
  (Default|EventHide (Variables|Default|GetBP_Hotspot))
  (Variables|/Game/Base/MotionControllerPawn/MotionControllerPawn.MotionControllerPawn_C|SetCanTPByController (Variables|Default|GetPawn) true)
  (Default|SetImage _pawnwbpfaceimg "/Game/Media/Photos/gamepad.gamepad")
  (Default|Show _pawnwbpfaceimg))

(event Custom|Event%20Init
  (EventDispatchers|BindEventtoFinishDispatcher (Variables|Default|GetBP_Test) (delegate Custom|TutorialTestCompleted))
  (EventDispatchers|BindEventtoActivateDispatcher (Variables|Default|GetBP_Hotspot) (delegate Custom|TutorialHotspotActivated)))

(event EventTick
  (params (DeltaSeconds :type Float%20%28single-precision%29))
  (|CallParentFunction DeltaSeconds))

(event EventPlayerEntered
  (params (MotionControllerPawn :type Motion%20Controller%20Pawn%20Object%20Reference))
  (bind _bp_test (Variables|Default|GetBP_Test))
  (|CallParentFunction 0)
  (Utilities|FlowControl|Sequence
    (:then_0
      (bind _output_get (Variables|Default|SetPawn MotionControllerPawn))
      (bind _aswbp_face_img (Utilities|Casting|CastToWBP_FaceImg (UserInterface|GetUserWidgetObject (Variables|/Game/Base/MotionControllerPawn/MotionControllerPawn.MotionControllerPawn_C|GetFaceImage _output_get))))
      (Variables|Default|SetPawnWBPFaceImg _aswbp_face_img))
    (:then_1
      (CallFunction|EventInit))
    (:then_2
      (|ShowLogos)
      (Default|EventStart _bp_test)
      (Default|EventOpen _bp_test))))

(event EventPlayerLeft
  (params (MotionControllerPawn :type Motion%20Controller%20Pawn%20Object%20Reference))
  (Default|Hide (Variables|Default|GetPawnWBPFaceImg) 4.0))

(fn ConstructionScript
  (|CallParentFunction))