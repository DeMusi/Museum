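; BP_HotSpot is a look-activated hotspot that moves the player to another scene after the gaze dwells on it.
; LookatStart shows a cylinder, starts a dwell timeline and animates the arrow box's position and roll through a second timeline.
; When the dwell timeline finishes forward, MotionControllerPawn executes the scene change to NextWorld with InitialRotation.
; LookatStop hides the cylinder and reverses both timelines, so only a completed forward run triggers travel.
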(event EventLookatStart
  (Utilities|FlowControl|Sequence
    (:then_0
      (Development|SetHiddeninGame (Variables|Default|GetCylinder) false false)
      (bind _direction (Timeline|Timeline_1 PlayFromStart)
        (:Finished
          (if (Utilities|Enum|Equal(Enum) _direction "Forward")
            (Default|ExecuteSceneChange (CallFunction|GetMotionControllerPawn) (Variables|Default|GetNextWorld) (Variables|Default|GetInitialRotation))))))
    (:then_1
      (bind _newtrack_0 (Timeline|ArrowTimeline Play) ; Location X, Location Z, Rotation X
        (:Update
          (Transformation|SetRelativeLocationAndRotation (Variables|Default|Getarrow_Box) (Math|Vector|MakeVector (.x _newtrack_0) 0.0 (.y _newtrack_0)) (Math|Rotator|MakeRotator (.z _newtrack_0) 0.0 9e+01) false false))))))

(event EventLookatStop
  (Utilities|FlowControl|Sequence
    (:then_0
      (Development|SetHiddeninGame (Variables|Default|GetCylinder) true false)
      (bind _direction (Timeline|Timeline_1 ReverseFromEnd)
        (:Finished
          (if (Utilities|Enum|Equal(Enum) _direction "Forward")
            (Default|ExecuteSceneChange (CallFunction|GetMotionControllerPawn) (Variables|Default|GetNextWorld) (Variables|Default|GetInitialRotation))))))
    (:then_1
      (bind _newtrack_0 (Timeline|ArrowTimeline Reverse) ; Location X, Location Z, Rotation X
        (:Update
          (Transformation|SetRelativeLocationAndRotation (Variables|Default|Getarrow_Box) (Math|Vector|MakeVector (.x _newtrack_0) 0.0 (.y _newtrack_0)) (Math|Rotator|MakeRotator (.z _newtrack_0) 0.0 9e+01) false false))))))

(fn ConstructionScript)

(fn GetMotionControllerPawn
  (bind _asmotion_controller_pawn (Utilities|Casting|CastToMotionControllerPawn (Game|Player|GetPlayerPawn 0)))
  (return _asmotion_controller_pawn))