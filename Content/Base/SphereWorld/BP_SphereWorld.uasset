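; BP_SphereWorld is a VR sphere environment that shows a texture on its mesh, with optional video and audio.
; MakeWorldFromTexture builds a dynamic M_SphereWorld material at construction and again on player entry.
; Entering also opens the video source, plays audio and yaws the pawn's VR origin by RotationOffset, while leaving stops both media.
; Tick pushes CurrentOpacity, which is set outside these graphs, into the material.
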(event Custom|PlayerEntered
  (params (MotionControllerPawn :type Motion%20Controller%20Pawn%20Object%20Reference))
  (bind _audio (Variables|Default|GetAudio))
  (Utilities|FlowControl|Sequence
    (:then_0
      (if (Utilities|IsValid (Variables|Default|GetVideoSource))
        (Media|MediaPlayer|OpenSource (Variables|Default|GetMediaPlayer) (Variables|Default|GetVideoSource))))
    (:then_1
      (CallFunction|MakeWorldfromTexture (Variables|Default|GetTexture)))
    (:then_2
      (if (Utilities|IsValid (Variables|/Script/Engine.AudioComponent|GetSound _audio))
        (Audio|Components|Audio|Play _audio 0.0)))
    (:then_3
      (Transformation|AddLocalRotation (Variables|/Game/Base/MotionControllerPawn/MotionControllerPawn.MotionControllerPawn_C|GetVROrigin MotionControllerPawn) (Math|Rotator|MakeRotator 0.0 0.0 (Variables|Default|GetRotationOffset)) false false))))

(event Custom|PlayerLeft
  (params (MotionControllerPawn :type Motion%20Controller%20Pawn%20Object%20Reference))
  (Audio|Components|Audio|Stop (Variables|Default|GetAudio))
  (Media|MediaPlayer|Close (Variables|Default|GetMediaPlayer) :!class /Script/MediaAssets.MediaPlayer))

(event EventTick
  (params (DeltaSeconds :type Float%20%28single-precision%29))
  (Rendering|Material|SetScalarParameterValue (Variables|Default|GetDynMat) "Opacity" (Variables|Default|GetCurrentOpacity) :!class /Script/Engine.MaterialInstanceDynamic))

(fn ConstructionScript
  (CallFunction|MakeWorldfromTexture (Variables|Default|GetTexture)))

(fn MakeWorldfromTexture
  (params (texture_source :type Texture%20Object%20Reference))
  (bind _returnvalue (Rendering|Material|CreateDynamicMaterialInstance "/Game/Base/SphereWorld/M_SphereWorld.M_SphereWorld" "None" :!class /Script/Engine.KismetMaterialLibrary))
  (Variables|Default|SetDynMat _returnvalue)
  (Utilities|FlowControl|Sequence
    (:then_0
      (Rendering|Material|SetTextureParameterValue (Variables|Default|GetDynMat) "Texture" texture_source))
    (:then_1
      (Rendering|Material|SetMaterial (Variables|Components|GetStaticMesh) 0 (Variables|Default|GetDynMat)))))