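; BP_IntroSphere is an introduction sphere that shows a video when the player enters, then moves on to the next scene.
; On entry it fires the motion controller pawn's watch-video event, waits a fixed delay, and has the pawn execute the scene change to NextScene.
; Leaving closes the media player, though nothing here cancels the pending change.
; Tick keeps playing an opacity timeline that updates CurrentOpacity.
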(event EventTick
  (params (DeltaSeconds :type Float%20%28single-precision%29))
  (|CallParentFunction 0.0)
  (bind _opacity (Timeline|OpacityTimeline Play)
    (:Update
      (Variables|Default|SetCurrentOpacity _opacity))))

(event EventPlayerEntered
  (|CallParentFunction)
  (bind _motioncontrollerpawn (CallFunction|GetMotionControllerPawn))
  (Default|EventWatchVideo _motioncontrollerpawn)
  (Utilities|FlowControl|Delay 1.3e+02)
  (bind _motioncontrollerpawn_2 (CallFunction|GetMotionControllerPawn))
  (Default|ExecuteSceneChange _motioncontrollerpawn_2 (Variables|Default|GetNextScene) 0.0))

(event EventPlayerLeft
  (|CallParentFunction)
  (Media|MediaPlayer|Close (Variables|Default|GetMediaPlayer2) :!class /Script/MediaAssets.MediaPlayer))

(fn ConstructionScript
  (|CallParentFunction))

(fn GetMotionControllerPawn
  (bind _asmotion_controller_pawn (Utilities|Casting|CastToMotionControllerPawn (Game|Player|GetPlayerPawn 0)))
  (return _asmotion_controller_pawn))