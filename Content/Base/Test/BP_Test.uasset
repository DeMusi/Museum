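; Timed quiz actor that shows questions on a widget component and takes answers through an array of answer button actors.
; The construction script loads questions from a DataTable, and BuildQuestion fills the buttons and refreshes progress.
; Correct answers add points and advance after a delay, while wrong ones subtract points.
; Timeout or the last question swaps in the finish widget and calls a dispatcher; timelines scale everything to open or close.
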(event Custom|Event%20Open
  (bind _defaultsceneroot (Variables|Components|GetDefaultSceneRoot))
  (Rendering|SetVisibility _defaultsceneroot true false)
  (bind _scale (Timeline|Timeline_0 PlayFromStart)
    (:Update
      (Transformation|SetWorldScale3D _defaultsceneroot (Math|Conversions|ToVector(Float) _scale))
      (for _array_element (Variables|Default|GetAnswerButtons)
        (Transformation|SetWorldScale3D (Variables|/Script/Engine.Actor|GetRootComponent _array_element) (Math|Conversions|ToVector(Float) _scale))))))

(event Custom|Event%20Finish
  (Variables|Default|SetIsPlaying false)
  (Rendering|SetVisibility (Variables|Components|GetTestWidget) false false)
  (Rendering|SetVisibility (Variables|Default|GetFinishWidget) true false)
  (CallFunction|HideAllButtons)
  (Default|CallFinishDispatcher))

(event Custom|Event%20Close
  (bind _defaultsceneroot (Variables|Components|GetDefaultSceneRoot))
  (bind _scale (Timeline|Timeline_1 PlayFromStart)
    (:Update
      (Transformation|SetWorldScale3D _defaultsceneroot (Math|Conversions|ToVector(Float) _scale))
      (for _array_element (Variables|Default|GetAnswerButtons)
        (Transformation|SetWorldScale3D (Variables|/Script/Engine.Actor|GetRootComponent _array_element) (Math|Conversions|ToVector(Float) _scale))))
    (:Finished
      (Rendering|SetVisibility _defaultsceneroot false false))))

(event Custom|Event%20Start
  (CallFunction|BuildQuestion)
  (Variables|Default|SetTimeLeft (Variables|Default|GetTestDuration))
  (Variables|Default|SetIsPlaying true))

(event Custom|Event%20Answer
  (params (Answer%20Index :type Integer))
  (bind _answerbuttons (Variables|Default|GetAnswerButtons))
  (bind _output (Utilities|Array|Get(acopy) _answerbuttons Answer%20Index))
  (if (|IsAnswerRight Answer%20Index)
    (Default|PlayCorrectAnimation _output)
    (Variables|Default|SetPoints (+ (Variables|Default|GetPoints) 10))
    (Utilities|FlowControl|Delay 1.0)
    (CallFunction|ToNextQuestion)
    (else
      (Default|PlayWrongAnimation _output)
      (Variables|Default|SetPoints (- (Variables|Default|GetPoints) 5)))))

(event EventBeginPlay
  (Utilities|FlowControl|Sequence
    (:then_0
      (bind _aswbp_test (Utilities|Casting|CastToWBP_Test (UserInterface|GetUserWidgetObject (Variables|Components|GetTestWidget))))
      (Variables|/Game/Base/Test/WBP_Test.WBP_Test_C|SetTestBP _aswbp_test self)
      (bind _aswbp_finish (Utilities|Casting|CastToWBP_Finish (UserInterface|GetUserWidgetObject (Variables|Default|GetFinishWidget))))
      (Variables|/Game/Base/Test/WBP_Finish.WBP_Finish_C|SetBP_Test _aswbp_finish self))
    (:then_1
      (for _array_element (Variables|Default|GetAnswerButtons)
        (Variables|/Game/Base/Test/BP_TestAnswer.BP_TestAnswer_C|SetBP_Test _array_element self)))
    (:then_2
      (if (Variables|Default|GetStart%20Closed)
        (CallFunction|EventClose)))))

(event EventTick
  (params (DeltaSeconds :type Float%20%28single-precision%29))
  (if (Variables|Default|GetIsPlaying)
    (Variables|Default|SetTimeLeft (- (Variables|Default|GetTimeLeft) DeltaSeconds))
    (if (< (Variables|Default|GetTimeLeft) 0.0)
      (CallFunction|EventFinish))))

(fn ConstructionScript
  (bind _testdatatable (Variables|Default|GetTestDataTable))
  (bind _outrownames (DataTable|GetDataTableRowNames _testdatatable))
  (for _array_element _outrownames
    (bind _returnvalue (Utilities|GetDataTableRow _testdatatable _array_element)
      (:then
        (Utilities|Array|Add (Variables|Default|GetQuestions) _returnvalue)))))

(fn BuildQuestion
  (Utilities|FlowControl|Sequence
    (:then_0
      (CallFunction|LookStopAllButtons))
    (:then_1
      (bind _output_get (Variables|Default|SetCurrentQuestion (Utilities|Array|Get(acopy) (Variables|Default|GetQuestions) (Variables|Default|GetCurrentQuestionIndex))))
      (Utilities|Array|Resize (.Answers (Utilities|Struct|BreakS_Question _output_get)) (Utilities|Array|Length (Variables|Default|GetAnswerButtons))))
    (:then_2
      (for (_array_element _array_index) (.Answers (Utilities|Struct|BreakS_Question _output_get))
        (Default|SetAnswer (Utilities|Array|Get(acopy) (Variables|Default|GetAnswerButtons) _array_index) _array_element _array_index)))
    (:then_3
      (|RefreshProgress))))

(fn LookStopAllButtons
  (for _array_element (Variables|Default|GetAnswerButtons)
    (Class|BPILookat|LookatStop(Message) _array_element)))

(fn ToNextQuestion
  (bind _result (Math|Integer|IncrementInt (Variables|Default|GetCurrentQuestionIndex))
    (:%20%20
      (if (>= _result (Utilities|Array|Length (Variables|Default|GetQuestions)))
        (CallFunction|EventFinish)
        (else
          (CallFunction|BuildQuestion))))))

(fn HideAllButtons
  (for _array_element (Variables|Default|GetAnswerButtons)
    (Rendering|SetActorHiddenInGame _array_element true)))