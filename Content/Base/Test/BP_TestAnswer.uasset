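; BP_TestAnswer is one selectable quiz answer, shown through a WBP_TestAnswer widget and chosen by sustained look-at.
; LookatStart plays the highlight and a timeline that sends AnswerIndex to BPTest when finished forward; LookatStop reverses both.
; SetAnswer stores text and index, hiding the widget for empty text, and separate functions play correct or wrong animations.
; Much older quiz logic remains as unconnected, never-run nodes.
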(event EventBeginPlay
  (bind _wbp_testanswer (CallFunction|GetWidget))
  (Variables|/Game/Base/Test/WBP_TestAnswer.WBP_TestAnswer_C|SetBP_TestAnswer _wbp_testanswer self))

(event EventLookatStart
  (bind _wbp_testanswer (CallFunction|GetWidget))
  (UserInterface|Animation|PlayAnimation _wbp_testanswer (Variables|/Game/Base/Test/WBP_TestAnswer.WBP_TestAnswer_C|GetHighlightAnimation _wbp_testanswer) 0.0 1 "Forward" 1.0)
  (bind _direction (Timeline|Timeline_1 Play)
    (:Finished
      (if (Utilities|Enum|Equal(Enum) _direction "Forward")
        (Default|EventAnswer (Variables|Default|GetBP_Test) (Variables|Default|GetAnswerIndex))))))

(event EventLookatStop
  (bind _wbp_testanswer (CallFunction|GetWidget))
  (UserInterface|Animation|PlayAnimation _wbp_testanswer (Variables|/Game/Base/Test/WBP_TestAnswer.WBP_TestAnswer_C|GetHighlightAnimation _wbp_testanswer) 0.0 1 "Reverse" 1.0)
  (bind _direction (Timeline|Timeline_1 Reverse)
    (:Finished
      (if (Utilities|Enum|Equal(Enum) _direction "Forward")
        (Default|EventAnswer (Variables|Default|GetBP_Test) (Variables|Default|GetAnswerIndex))))))

(fn ConstructionScript)

(fn SetAnswer
  (params (Text :type String) (Index :type Integer))
  (bind _output_get (Variables|Default|SetAnswerText Text))
  (Rendering|SetVisibility (Variables|Components|GetWidget) (Utilities|Enum|NotEqual(Enum) _output_get "") false)
  (Variables|Default|SetAnswerIndex Index))

(fn PlayCorrectAnimation
  (bind _wbp_testanswer (CallFunction|GetWidget))
  (UserInterface|Animation|PlayAnimation _wbp_testanswer (Variables|/Game/Base/Test/WBP_TestAnswer.WBP_TestAnswer_C|GetCorrectAnimation _wbp_testanswer) 0.0 1 "Forward" 1.0))

(fn GetWidget
  (bind _aswbp_test_answer (Utilities|Casting|CastToWBP_TestAnswer (UserInterface|GetUserWidgetObject (Variables|Components|GetWidget))))
  (return _aswbp_test_answer))

(fn PlayWrongAnimation
  (bind _wbp_testanswer (CallFunction|GetWidget))
  (UserInterface|Animation|PlayAnimation _wbp_testanswer (Variables|/Game/Base/Test/WBP_TestAnswer.WBP_TestAnswer_C|GetWrongAnimation _wbp_testanswer) 0.0 1 "Forward" 1.0))